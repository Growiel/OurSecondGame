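; BP_Porte is an interactable door that opens only when the player carries a required item.
; On Interact it casts the instigator to Main_Character and checks its inventory for the NeededItem row name.
; If the item is present, it stores the door mesh's current relative rotation and plays a timeline that lerps it 90 degrees further in yaw.
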(event `InteractableInterface.Interact`
  (params (InteractedBy :type "Actor Object Reference"))
  (bind _newvar_0 (`self.NewVar_0`))
  (bind (_neededitem_datatable _neededitem_rowname) (break `DataTableRowHandle` (`self.NeededItem`)))
  (bind _asmain_character (cast `/Game/Character/Blueprints/Main_Character` InteractedBy))
  (if (`OurSecondGameCharacter.IsInInventory` _asmain_character _neededitem_rowname)
    (set `self.NewVar_0` (`SceneComponent.RelativeRotation` (`self.SM_Door`)))
    (bind (_direction _newtrack_0) (`Timeline|Timeline_0` :!via `PlayFromStart`)
      (:`Update`
        (`SceneComponent.K2_SetRelativeRotation` (`self.SM_Door`) (`KismetMathLibrary.RLerp` _newvar_0 (`KismetMathLibrary.MakeRotator` (.roll _newvar_0) (.pitch _newvar_0) (+ (.yaw _newvar_0) 90.0)) _newtrack_0) false false)))))

(fn `UserConstructionScript`)