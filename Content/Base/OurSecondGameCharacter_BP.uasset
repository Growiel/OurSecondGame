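; Player character Blueprint that adds an action bar HUD and a toggleable inventory screen.
; BeginPlay creates both widgets, and showing the inventory pauses the game, enables the cursor and swaps out the HUD.
; Four action bar inputs index into the AvailableActions keys to toggle the lamp's spotlight, if owned, or run a placeholder compass action.
; ToggleEnableAction updates that map and rebuilds the bar's buttons.
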(event `InputAction|ActionBar1`
  (params (Key :type "Key Structure" :default "AnyKey"))
  ;[1 1 1] Bind ActionBar inputs
  (:`Pressed`
    (`self.HandleActions` 0)))

(event `InputAction|ActionBar2`
  (params (Key :type "Key Structure" :default "AnyKey"))
  ;[1 1 1] Bind ActionBar inputs
  (:`Pressed`
    (`self.HandleActions` 1)))

(event `InputAction|ActionBar3`
  (params (Key :type "Key Structure" :default "AnyKey"))
  ;[1 1 1] Bind ActionBar inputs
  (:`Pressed`
    (`self.HandleActions` 2)))

(event `InputAction|ActionBar4`
  (params (Key :type "Key Structure" :default "AnyKey"))
  ;[1 1 1] Bind ActionBar inputs
  (:`Pressed`
    (`self.HandleActions` 3)))

(event `self.ReceiveBeginPlay`
  (bind _returnvalue (`GameplayStatics.GetPlayerController` 0))
  (`|ExecutionSequence`
    (:`then_0`
      ;[1 1 1] Add the Actionbar UMG to the screen
      (bind _returnvalue_2 (`|CreateWidget` "/Game/HUD.HUD_C" _returnvalue))
      (bind _output_get (set `self.HUD UMG` _returnvalue_2))
      (set `self.ActionBarUMG` (`/Game/HUD.ActionBar_111` _output_get))
      (`UserWidget.AddToViewport` _output_get 0))
    (:`then_1`
      ;[1 1 1] Create InventoryUMG, do not show on screen
      (bind _returnvalue_3 (`|CreateWidget` "/Game/Inventory/UMG/Inventory.Inventory_C" _returnvalue))
      (set `self.Inventory UMG` _returnvalue_3))))

(event `InputAction|ToggleInventory` :paused true
  (params (Key :type "Key Structure" :default "AnyKey"))
  ;[1 1 1] Toggle Inventory
  (:`Pressed`
    (`/Engine/EditorBlueprintResources/StandardMacros.FlipFlop`
      (:`A`
        (`self.ShowInventory`))
      (:`B`
        (`self.HideInventory`)))))

(fn `HandleActions`
  (params (ActionIndex :type Integer))
  (bind _keys (`BlueprintMapLibrary.Map_Keys` (`self.AvailableActions`)))
  (switch `name` (`|GetArrayItem` _keys ActionIndex)
    (:`lamp`
      (`self.HandleLamp`))
    (:`compass`
      (`KismetSystemLibrary.PrintString` "Here we would do things with the compass"))))

(fn `HandleLamp`
  (locals (LampItemHandle :type "DataTableRowHandle Structure" :default (struct :`DataTable` "DataTable'/Game/Inventory/ItemData_DataTable.ItemData_DataTable'" :`RowName` "lamp")))
  (bind (_lampitemhandle_datatable _lampitemhandle_rowname) (break `DataTableRowHandle` (`local.LampItemHandle`)))
  ;[1 1 1] Check that we do have the lamp
  (if (`self.IsInInventory` _lampitemhandle_rowname)
    ;[1 1 1] Toggle on/off
    (bind _output_get (set `self.IsLampTorchOff?` (not (`self.IsLampTorchOff?`))))
    (`SceneComponent.SetHiddenInGame` (`self.SpotLight`) _output_get false)
    (return)
    (else
      (return))))

(fn `HideInventory`
  (bind _returnvalue (`GameplayStatics.GetPlayerController` 0))
  (`|ExecutionSequence`
    (:`then_0`
      (`Widget.RemoveFromParent` (`self.Inventory UMG`)))
    (:`then_1`
      (set `PlayerController.bShowMouseCursor` false _returnvalue)
      (`WidgetBlueprintLibrary.SetInputMode_GameOnly` _returnvalue)
      (`GameplayStatics.SetGamePaused` false))
    (:`then_2`
      (`UserWidget.AddToViewport` (`self.HUD UMG`) 0))
    (:`then_3`
      (return))))

(fn `ShowInventory`
  (bind _returnvalue (`GameplayStatics.GetPlayerController` 0))
  (`|ExecutionSequence`
    (:`then_0`
      (`UserWidget.AddToViewport` (`self.Inventory UMG`) 0))
    (:`then_1`
      (set `PlayerController.bShowMouseCursor` true _returnvalue)
      (`WidgetBlueprintLibrary.SetInputMode_GameAndUIEx` _returnvalue (`self.Inventory UMG`))
      (`GameplayStatics.SetGamePaused` true)
      (`/Game/Inventory/UMG/Inventory.Show` (`self.Inventory UMG`)))
    (:`then_2`
      (`Widget.RemoveFromParent` (`self.HUD UMG`)))
    (:`then_3`
      (return))))

(fn `ToggleEnableAction`
  (params (ActionName :type Name) (Enable :type Boolean))
  (`BlueprintMapLibrary.Map_Add` (`self.AvailableActions`) ActionName Enable)
  (`/Game/ActionBar/UMG/ActionBar.createButtons` (`self.ActionBarUMG`)))

(fn `UserConstructionScript`)